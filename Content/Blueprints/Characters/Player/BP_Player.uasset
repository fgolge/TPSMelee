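; Player character Blueprint whose graphs hold only on-screen debug output, with no gameplay logic.
; Tick prints the current weapon state every frame, using a fixed key so the message updates in place.
; Similar keyed prints for health, alive status, combat and action states, movement speed and location sit unconnected and never run.
; BeginPlay, overlap and the construction script do nothing.
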(event EventBeginPlay)

(event Collision|EventActorBeginOverlap
  (params (OtherActor :type Actor%20Object%20Reference)))

(event EventTick
  (params (DeltaSeconds :type Float%20%28single-precision%29))
  (Utilities|FlowControl|Sequence ; Debug
    (:then_0
      (Development|PrintString (Utilities|String|EnumtoString (Class|BasePlayer|GetWeaponState)) true true "(R=0.000000,G=0.660000,B=1.000000,A=1.000000)" 2.0 "0"))
    (:then_1)
    (:then_2)
    (:then_3)
    (:then_4)
    (:then_5)
    (:then_6)
    (:then_7)))

(fn ConstructionScript)